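; Finish line actor that reports a lap to the race manager when an actor crosses its trigger moving forward.
; On overlap, it dots the actor's normalized velocity with its own forward vector to reject backward or sideways crossings.
; A single DoOnce gates the OnLapPassedMessage sent to BP_RaceManager, so further crossings are ignored until ResetFinishLine re-arms it.
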(event `self.Finish line Trigger.OnComponentBeginOverlap`
  (params (OverlappedComponent :type "PrimitiveComponent Object Reference") (OtherActor :type "Actor Object Reference") (OtherComp :type "PrimitiveComponent Object Reference") (OtherBodyIndex :type Integer) (bFromSweep :type Boolean) (SweepResult :type "HitResult Structure (by ref)"))
  ; Checks which actor is passing through it, sets it as a ship ref and sends it as a message to the Race Manager, so it can manage the lap and all that
  (if (> (`KismetMathLibrary.Dot_VectorVector` (`KismetMathLibrary.Normal` (`self.GetVelocity` OtherActor)) (`self.GetActorForwardVector`)) 0.1)
    (`/Engine/EditorBlueprintResources/StandardMacros.DoOnce` false :!label _label
      (:`Completed`
        (bind _returnvalue (`GameplayStatics.GetActorOfClass` "/Game/Blueprints/Managers/BP_RaceManager.BP_RaceManager_C"))
        (message `/Game/Blueprints/Finish_Line/BPI_Racing.On Lap Passed` _returnvalue OtherActor)
        (`KismetSystemLibrary.PrintString` "Lap Completed")))))

(event `/Game/Blueprints/Finish_Line/BPI_Racing.Reset Finish Line`
  ; Checks which actor is passing through it, sets it as a ship ref and sends it as a message to the Race Manager, so it can manage the lap and all that
  (goto _label :!via `Reset`))

(fn `UserConstructionScript`)