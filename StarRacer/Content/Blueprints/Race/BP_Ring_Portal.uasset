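; BP_Ring_Portal is a checkpoint ring in a spaceship race.
; When a non-respawning ship overlaps its box moving along the ring's forward vector, it calls ValidateRing on the race manager and saves its transform as the ship's last checkpoint.
; The manager's current ring index is passed, not one owned by the ring.
; A DoOnce gates triggers, resetting shortly after a forward pass only.
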(event `self.ReceiveBeginPlay`
  (bind _returnvalue (`GameplayStatics.GetActorOfClass` "/Game/Blueprints/Managers/BP_RaceManager.BP_RaceManager_C"))
  (set `self.Race Manager Ref` _returnvalue))

(event `self.Box.OnComponentBeginOverlap`
  (params (OverlappedComponent :type "PrimitiveComponent Object Reference") (OtherActor :type "Actor Object Reference") (OtherComp :type "PrimitiveComponent Object Reference") (OtherBodyIndex :type Integer) (bFromSweep :type Boolean) (SweepResult :type "HitResult Structure (by ref)"))
  (bind _race_manager_ref (`self.Race Manager Ref`))
  ; Resets the finish line once the player passes a checkpoint
  (bind _asbp_spaceship (cast `/Game/Blueprints/SpaceShip/BP_Spaceship` OtherActor))
  (if (not (`/Game/Blueprints/SpaceShip/BP_Spaceship.Is Respawning` _asbp_spaceship))
    (`/Engine/EditorBlueprintResources/StandardMacros.DoOnce` false :!label _label
      (:`Completed`
        (if (> (`KismetMathLibrary.Dot_VectorVector` (`KismetMathLibrary.Normal` (`self.GetVelocity` OtherActor)) (`self.GetActorForwardVector`)) 0.1)
          (bind _asbp_spaceship_2 (cast `/Game/Blueprints/SpaceShip/BP_Spaceship` OtherActor))
          (`/Game/Blueprints/Managers/BP_RaceManager.Validate Ring` _race_manager_ref (`/Game/Blueprints/Managers/BP_RaceManager.Current Ring Index` _race_manager_ref) _asbp_spaceship_2)
          (set `/Game/Blueprints/SpaceShip/BP_Spaceship.Last Checkpoint Transform` (`self.GetTransform`) _asbp_spaceship_2)
          (`KismetSystemLibrary.Delay` 0.2)
          (goto _label :!via `Reset`))))))

(fn `UserConstructionScript`)