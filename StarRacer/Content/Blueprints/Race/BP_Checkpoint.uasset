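; BP_Checkpoint is a race checkpoint that records a respawn-style transform on the spaceship passing through it.
; Its trigger overlap accepts only actors moving along the checkpoint's forward vector, tested by a dot product on normalized velocity.
; A valid pass resets the finish line message on FinishLineRef, then stores the checkpoint's transform as the BP_Spaceship's LastCheckpointTransform.
; The message reset precedes the cast, so any forward-moving actor triggers it.
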(event `self.Checkpoint Trigger.OnComponentBeginOverlap`
  (params (OverlappedComponent :type "PrimitiveComponent Object Reference") (OtherActor :type "Actor Object Reference") (OtherComp :type "PrimitiveComponent Object Reference") (OtherBodyIndex :type Integer) (bFromSweep :type Boolean) (SweepResult :type "HitResult Structure (by ref)"))
  ; Resets the finish line once the player passes a checkpoint
  (if (> (`KismetMathLibrary.Dot_VectorVector` (`KismetMathLibrary.Normal` (`self.GetVelocity` OtherActor)) (`self.GetActorForwardVector`)) 0.1)
    (message `/Game/Blueprints/Race/BPI_Racing.Reset Finish Line` (`self.Finish Line Ref`))
    (bind _asbp_spaceship (cast `/Game/Blueprints/SpaceShip/BP_Spaceship` OtherActor))
    (set `/Game/Blueprints/SpaceShip/BP_Spaceship.Last Checkpoint Transform` (`self.GetTransform`) _asbp_spaceship)))

(fn `UserConstructionScript`)