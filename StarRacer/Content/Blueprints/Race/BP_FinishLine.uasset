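; BP_FinishLine is the race finish line trigger that reports passing actors to BP_RaceManager for lap tracking.
; On overlap, a dot product of the actor's velocity and the line's forward vector filters out wrong-way crossings.
; Valid crossings pass a shared DoOnce, wait briefly, send OnLapPassedMessage, then reset the gate, so overlaps during the delay are ignored.
; The manager reference cached on BeginPlay feeds only unconnected logic.
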(event `self.ReceiveBeginPlay`
  (bind _returnvalue (`GameplayStatics.GetActorOfClass` "/Game/Blueprints/Managers/BP_RaceManager.BP_RaceManager_C"))
  (set `self.Race Manager Ref` _returnvalue))

(event `self.Finish line Trigger.OnComponentBeginOverlap`
  (params (OverlappedComponent :type "PrimitiveComponent Object Reference") (OtherActor :type "Actor Object Reference") (OtherComp :type "PrimitiveComponent Object Reference") (OtherBodyIndex :type Integer) (bFromSweep :type Boolean) (SweepResult :type "HitResult Structure (by ref)"))
  ; Checks which actor is passing through it, sets it as a ship ref and sends it as a message to the Race Manager, so it can manage the lap and all that
  (if (> (`KismetMathLibrary.Dot_VectorVector` (`KismetMathLibrary.Normal` (`self.GetVelocity` OtherActor)) (`self.GetActorForwardVector`)) 0.1)
    (`/Engine/EditorBlueprintResources/StandardMacros.DoOnce` false :!label _label
      (:`Completed`
        (bind _returnvalue (`GameplayStatics.GetActorOfClass` "/Game/Blueprints/Managers/BP_RaceManager.BP_RaceManager_C"))
        (`KismetSystemLibrary.Delay` 0.2)
        (message `/Game/Blueprints/Race/BPI_Racing.On Lap Passed` _returnvalue OtherActor)
        (goto _label :!via `Reset`)))))

(fn `UserConstructionScript`)