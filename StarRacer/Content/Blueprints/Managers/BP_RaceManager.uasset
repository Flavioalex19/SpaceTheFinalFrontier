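; BP_RaceManager is a race manager that counts laps per ship and detects when the race is finished.
; On BeginPlay it casts the first player's pawn to BP_Spaceship and stores it as PlayerRef.
; OnLapPassed increments the given ship's count in the LapTracker map, then prints a finish message once that count reaches TotalLaps.
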(event `self.ReceiveBeginPlay`
  (bind _asbp_spaceship (cast `/Game/Blueprints/SpaceShip/BP_Spaceship` (`GameplayStatics.GetPlayerPawn` 0)))
  (set `self.Player Ref` _asbp_spaceship))

(event `/Game/Blueprints/Finish_Line/BPI_Racing.On Lap Passed`
  (params (`Ship Ref` :type "Actor Object Reference"))
  ; Add 1+ on lap
  (bind _result (`/Engine/EditorBlueprintResources/StandardMacros.IncrementInt` (`BlueprintMapLibrary.Map_Find` (`self.Lap Tracker`) `Ship Ref`))
    (:`  `
      (bind _output_get (set `self.Current Laps` _result))
      (`BlueprintMapLibrary.Map_Add` (`self.Lap Tracker`) `Ship Ref` _result)
      (if (>= _output_get (`self.Total Laps`))
        (`KismetSystemLibrary.PrintString` "Race Finished!")))))

(fn `UserConstructionScript`)